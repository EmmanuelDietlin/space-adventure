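; Player controller Blueprint that lets a controlled SpaceEntity pawn interact with actors in front of it.
; On BeginPlay it binds a handler to its OnInteract dispatcher.
; The handler line-traces on the Visibility channel from the pawn's HeadComponent along the pawn's forward vector for InteractDistance, ignoring the pawn.
; It then calls InteractMessage on the hit actor, without checking whether the trace hit anything.
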(event `self.ReceiveBeginPlay`
  (add `self.OnInteract` (delegate `OnInteract_Event`)))

(event `OnInteract_Event`
  (bind _returnvalue (`self.K2_GetPawn`))
  (bind _asspace_entity (cast `SpaceEntity` _returnvalue))
  (bind _headcomponent (`SpaceEntity.HeadComponent` _asspace_entity))
  (`/Engine/EditorBlueprintResources/StandardMacros.IsValid` _headcomponent
    (:`Is Valid`
      (bind _returnvalue_location (`KismetMathLibrary.BreakTransform` (`SceneComponent.K2_GetComponentToWorld` _headcomponent)))
      (bind _outhit (`KismetSystemLibrary.LineTraceSingle` _returnvalue_location (+ _returnvalue_location (* (`self.GetActorForwardVector` _returnvalue) (`self.InteractDistance`))) "TraceTypeQuery1" false (`|MakeArray` _returnvalue :!type "Actor Object Reference")))
      (bind _output_get (set `self.InteractActor` (`.HitActor` (`GameplayStatics.BreakHitResult` _outhit))))
      (message `Interactable.Interact` _output_get))))

(fn `UserConstructionScript`)